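; BP_Chest is an interactable chest opened by holding interact until a SearchWidget progress bar fills.
; Overlap toggles the widget's visibility and interact begin/end drives its progress, all gated by a Closed macro checking the Open flag.
; OpenChest sets Open, hides the widget, shows a point light, spawns a Niagara effect and plays a timeline intended to rotate the lid.
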(event EventOnInteractBegin
  ;[1 1 1] Hold E
  (Utilities|Closed
    (:true
      (bind _assearch_widget (Utilities|Casting|CastToSearchWidget (UserInterface|GetUserWidgetObject (Variables|Default|GetWidget))))
      (Default|BeginProgress _assearch_widget))))

(event EventOnInteractEnd
  ;[1 1 1] Hold E
  (Utilities|Closed
    (:true
      (bind _assearch_widget (Utilities|Casting|CastToSearchWidget (UserInterface|GetUserWidgetObject (Variables|Default|GetWidget))))
      (Default|EndProgress _assearch_widget))))

(event EventBeginPlay
  ;[1 1 1] Open Chest Action
  (bind _assearch_widget (Utilities|Casting|CastToSearchWidget (UserInterface|GetUserWidgetObject (Variables|Default|GetWidget))))
  (Variables|/Game/Blueprints/Items/SearchWidget.SearchWidget_C|SetRequiredHoldTime _assearch_widget 1.25)
  (EventDispatchers|AssignOnProgressBarFull _assearch_widget (EventDispatchers|CreateEvent :!event OpenChest)))

(event EventOnOverlapBegin
  ;[1 1 1] Overlap Visibility
  (Utilities|Closed
    (:true
      (Rendering|SetVisibility (Variables|Default|GetWidget) true false))))

(event EventOnOverlapEnd
  ;[1 1 1] Overlap Visibility
  (Utilities|Closed
    (:true
      (Rendering|SetVisibility (Variables|Default|GetWidget) false false))))

(fn ConstructionScript)

(fn OpenChest
  (Utilities|Closed
    (:true
      (Variables|Private|SetOpen? true)
      (Rendering|SetVisibility (Variables|Default|GetWidget) false false)
      (Rendering|SetVisibility (Variables|Default|GetPointLight) true false)
      (Niagara|SpawnSystematLocation "/Game/Blueprints/Items/NS_ChestOpen.NS_ChestOpen" (Transformation|GetActorLocation))
      (Components|Timeline|PlayfromStart (Variables|Default|GetOpenChestTimeline)))))