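; Key pickup actor that lowers the game mode's KeysLeft count, shows a KeyWidget on screen and destroys itself.
; Anything overlapping its Box collects it immediately with a 2D equip sound, as no actor filter is applied.
; A Machete_BP_MASTER overlapping the actor also enables player input, allowing silent collection by left click until the overlap ends.
; An attraction timeline that would lerp ItemKey toward the actor's location is present but never runs.
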(event OnComponentBeginOverlap(Box)
  (params (OverlappedComponent :type Primitive%20Component%20Object%20Reference) (OtherActor :type Actor%20Object%20Reference) (OtherComp :type Primitive%20Component%20Object%20Reference) (OtherBodyIndex :type Integer) (bFromSweep :type Boolean) (SweepResult :type Hit%20Result%20Structure%20%28by%20ref%29))
  ;[1 1 1] Get Key (Overlap)
  (bind _asgamemode_master (Utilities|Casting|CastToGamemode_MASTER (Game|GetGameMode)))
  (bind _result (Math|Integer|DecrementInt (Variables|/Game/Maps/Gamemode_MASTER.Gamemode_MASTER_C|GetKeysLeft _asgamemode_master))
    (:%20%20
      (Variables|/Game/Maps/Gamemode_MASTER.Gamemode_MASTER_C|SetKeysLeft _asgamemode_master _result)
      (bind _returnvalue (UserInterface|CreateWidget "/Game/ProgrammingStephanieB/KeyWidget.KeyWidget_C"))
      (UserInterface|Viewport|AddtoViewport _returnvalue 0)
      (Audio|PlaySound2D "/Game/Audio/Sound_Effects/Items/Item_Equip.Item_Equip" 1.0 1.0 0.0 0 0)
      (Actor|DestroyActor))))

(event Collision|EventActorBeginOverlap
  (params (OtherActor :type Actor%20Object%20Reference))
  ;[1 1 1] Collision settings(?)
  (Utilities|Casting|CastToMachete_BP_MASTER OtherActor)
  (Input|EnableInput (Game|GetPlayerController 0)))

(event Collision|EventActorEndOverlap
  (params (OtherActor :type Actor%20Object%20Reference))
  ;[1 1 1] Collision settings(?)
  (Utilities|Casting|CastToMachete_BP_MASTER OtherActor)
  (Input|DisableInput (Game|GetPlayerController 0)))

(event Input|MouseEvents|LeftMouseButton
  (params (Key :type Key%20Structure :default "None"))
  ;[1 1 1] Get Key (Left Click)
  (:Pressed
    (bind _asgamemode_master (Utilities|Casting|CastToGamemode_MASTER (Game|GetGameMode)))
    (bind _result (Math|Integer|DecrementInt (Variables|/Game/Maps/Gamemode_MASTER.Gamemode_MASTER_C|GetKeysLeft _asgamemode_master))
      (:%20%20
        (Variables|/Game/Maps/Gamemode_MASTER.Gamemode_MASTER_C|SetKeysLeft _asgamemode_master _result)
        (bind _returnvalue (UserInterface|CreateWidget "/Game/ProgrammingStephanieB/KeyWidget.KeyWidget_C"))
        (UserInterface|Viewport|AddtoViewport _returnvalue 0)
        (Actor|DestroyActor)))))

(fn ConstructionScript)