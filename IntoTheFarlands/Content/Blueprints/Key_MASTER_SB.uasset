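; Key_MASTER_SB is a key pickup actor that is collected with a left mouse click while in range.
; Overlap begin and end, filtered by a cast on the other actor, toggle the key's input from player controller 0.
; A click casts to Gamemode_MASTER, decrements and then zeroes KeysLeft, adds a widget to the viewport and destroys the key.
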(event Collision|EventActorBeginOverlap
  (params (OtherActor :type Actor%20Object%20Reference))
  (Utilities|Casting|CastTo OtherActor)
  (Input|EnableInput (Game|GetPlayerController 0)))

(event Collision|EventActorEndOverlap
  (params (OtherActor :type Actor%20Object%20Reference))
  (Utilities|Casting|CastTo OtherActor)
  (Input|DisableInput (Game|GetPlayerController 0)))

(event Input|MouseEvents|LeftMouseButton
  (params (Key :type Key%20Structure))
  (:Pressed
    (Utilities|Casting|CastToGamemode_MASTER (Game|GetGameMode))
    (Math|Integer|DecrementInt (Variables|Default|GetKeysLeft)
      (:%20%20
        (Variables|Default|SetKeysLeft 0)
        (bind _returnvalue (UserInterface|CreateWidget 0))
        (UserInterface|Viewport|AddtoViewport _returnvalue 0)
        (Actor|DestroyActor)))))

(fn ConstructionScript)