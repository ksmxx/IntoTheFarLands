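; Player character Blueprint for Machete, handling movement, look, jump, crouch, sprint, melee, NPC dialogue and damage.
; Tick uses Delay to drain or regenerate stamina roughly each second; exhaustion while sprinting zeroes walk speed until sprint is released.
; E triggers dialogue on the first overlapping NPC_Interact actor.
; Raw key presses play slash, run and walk montages; damage lowers health and plays the zombie death montage, even on non-lethal hits.
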(event EventTick
  (params (DeltaSeconds :type Float%20%28single-precision%29))
  (Utilities|FlowControl|Sequence
    (:then_0
      ;[1 1 1] Stamina Drain + Regen
      (if (Variables|Default|GetIsSprinting?)
        (Utilities|FlowControl|Delay 1.0)
        (if (<= (Variables|Default|GetStamina) 0)
          (Variables|Default|SetIsSprinting? false)
          (Variables|/Script/Engine.CharacterMovementComponent|SetMaxWalkSpeed (Variables|Character|GetCharacterMovement) 0.0)
          (else
            (Variables|Default|SetStamina (- (Variables|Default|GetStamina) 10))))
        (else
          (Utilities|FlowControl|Delay 1.0)
          (if (< (Variables|Default|GetStamina) (Variables|Default|GetMax%20Stamina))
            (Variables|Default|SetStamina (+ (Variables|Default|GetStamina) 8))))))))

(event Game|Damage|EventAnyDamage
  (params (Damage :type Float%20%28single-precision%29) (DamageType :type Damage%20Type%20Object%20Reference) (InstigatedBy :type Controller%20Object%20Reference) (DamageCauser :type Actor%20Object%20Reference))
  (bind _output_get (Variables|Default|SetHealth (- (Variables|Default|GetHealth) Damage)))
  (if (<= _output_get 0.0)
    (Utilities|FlowControl|DoOnce false
      (:Completed
        (Animation|PlayAnimMontage "/Game/3D_Objects/Characters/Machete/Animation/Zombie_Death_Anim_Montage.Zombie_Death_Anim_Montage" 1.0 "None")))
    (else
      (Animation|PlayAnimMontage "/Game/3D_Objects/Characters/Machete/Animation/Zombie_Death_Anim_Montage.Zombie_Death_Anim_Montage" 1.0 "None"))))

(event Input|ActionEvents|InputActionJumpAction
  (params (Key :type Key%20Structure))
  ;[1 1 1] Jumping
  (:Pressed
    (Character|Jump))
  (:Released
    (Character|StopJumping)))

(event Input|ActionEvents|InputActionCrouchAction
  (params (Key :type Key%20Structure))
  ;[1 1 1] Crouch
  (:Pressed
    (Character|Crouch)
    (Variables|Default|SetIsCrouching? true))
  (:Released
    (Character|UnCrouch)
    (Variables|Default|SetIsCrouching? false)))

(event Input|ActionEvents|InputActionSprintAction
  (params (Key :type Key%20Structure))
  ;[1 1 1] Sprinting
  (:Pressed
    (if (>= (Variables|Default|GetStamina) 1)
      (Variables|Default|SetIsSprinting? true)
      (Variables|/Script/Engine.CharacterMovementComponent|SetMaxWalkSpeed (Variables|Character|GetCharacterMovement) 1.2e+03)))
  (:Released
    (Variables|/Script/Engine.CharacterMovementComponent|SetMaxWalkSpeed (Variables|Character|GetCharacterMovement) 6e+02)
    (Variables|Default|SetIsSprinting? false)))

(event Input|AxisEvents|InputAxisLookLeft/Right
  (params (AxisValue :type Float%20%28single-precision%29))
  ;[1 1 1] Look Around
  (Pawn|Input|AddControllerYawInput AxisValue))

(event Input|AxisEvents|InputAxisMoveForward/Backwards
  (params (AxisValue :type Float%20%28single-precision%29))
  (Pawn|Input|AddMovementInput (Math|Vector|GetForwardVector (Math|Rotator|MakeRotator 0.0 0.0 (.Yaw (Math|Rotator|BreakRotator (Pawn|GetControlRotation :!class /Script/Engine.Pawn))))) AxisValue false))

(event Input|AxisEvents|InputAxisMoveRight/Left
  (params (AxisValue :type Float%20%28single-precision%29))
  (Pawn|Input|AddMovementInput (Math|Vector|GetRightVector (Math|Rotator|MakeRotator 0.0 0.0 (.Yaw (Math|Rotator|BreakRotator (Pawn|GetControlRotation :!class /Script/Engine.Pawn))))) AxisValue false))

(event Input|AxisEvents|InputAxisLookUp/Down
  (params (AxisValue :type Float%20%28single-precision%29))
  ;[1 1 1] Look Around
  (Pawn|Input|AddControllerPitchInput AxisValue))

(event Input|KeyboardEvents|E
  (params (Key :type Key%20Structure))
  ;[1 1 1] NPC Interact
  (:Pressed
    (bind _array_element (Utilities|Array|ForEachLoopwithBreak (Collision|GetOverlappingActors "/Script/Engine.Actor" :!class /Script/Engine.Actor) :!label _label)
      (:LoopBody
        (if (Utilities|DoesObjectImplementInterface _array_element "/Game/3D_Objects/Characters/NPC_Interact.NPC_Interact_C")
          (Class|NPCInteract|ActivateDialogue(Message) _array_element)
          (goto _label Break))))))

(event Input|MouseEvents|LeftMouseButton
  (params (Key :type Key%20Structure))
  ;[1 1 1] Sword Attack
  (:Pressed
    (Animation|PlayAnimMontage "/Game/3D_Objects/Characters/Machete/Animation/Sword_And_Shield_Slash_Montage.Sword_And_Shield_Slash_Montage" 1.0 "None")))

(event Input|KeyboardEvents|LeftShift
  (params (Key :type Key%20Structure))
  (:Pressed
    (Animation|PlayAnimMontage "/Game/3D_Objects/Characters/Machete/Animation/Standard_Run_Anim_Montage.Standard_Run_Anim_Montage" 1.0 "None")))

(event Input|KeyboardEvents|W
  (params (Key :type Key%20Structure))
  (:Pressed
    (Animation|PlayAnimMontage "/Game/3D_Objects/Characters/Machete/Animation/Walking_Montage.Walking_Montage" 1.0 "None")))

(fn ConstructionScript)